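; Openable door actor that swings around its yaw axis when its OpenDoor member fires OnOpen or OnClose.
; A timeline adds an animated Z angle to the rotation cached at BeginPlay, playing forward to open and reversing to close.
; A timeline event track plays the opening sound at the door's location, while a closing creak sound node is left unconnected.
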(event OnClose(OpenDoor)
  (bind _changeanglez (Timeline|Timeline_0 Reverse)
    (:Update
      (Transformation|SetActorRotation (Math|Rotator|CombineRotators (Variables|Default|GetInitialRotation) (Math|Rotator|MakeRotator 0.0 0.0 _changeanglez))))
    (:Sound%20Playing
      (Audio|PlaySoundatLocation "/Game/Audio/open_door_2.open_door_2" (Transformation|GetActorLocation) "0, 0, 0" 1.0 1.0 0.0 0 0 0))))

(event OnOpen(OpenDoor)
  (bind _changeanglez (Timeline|Timeline_0 Play)
    (:Update
      (Transformation|SetActorRotation (Math|Rotator|CombineRotators (Variables|Default|GetInitialRotation) (Math|Rotator|MakeRotator 0.0 0.0 _changeanglez))))
    (:Sound%20Playing
      (Audio|PlaySoundatLocation "/Game/Audio/open_door_2.open_door_2" (Transformation|GetActorLocation) "0, 0, 0" 1.0 1.0 0.0 0 0 0))))

(event EventBeginPlay
  (Variables|Default|SetInitialRotation (Transformation|GetActorRotation)))

(fn ConstructionScript)